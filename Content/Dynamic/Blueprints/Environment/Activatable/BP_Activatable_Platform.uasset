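; An activatable moving platform that travels between start and target location components when triggered.
; After a short delay, each activation alternates through a FlipFlop, playing audio while a timeline lerps the static mesh's world location.
; The LongLift flag selects which timeline drives forward movement.
; The return always reverses the UPDown timeline, even for long lifts.
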(event EventBeginPlay)

(event Collision|EventActorBeginOverlap
  (params (OtherActor :type Actor%20Object%20Reference)))

(event EventTick
  (params (DeltaSeconds :type Float%20%28single-precision%29)))

(event EventActivate/Deactivate
  (bind _audio (Variables|Default|GetAudio))
  (Utilities|FlowControl|Delay 2.0)
  (Utilities|FlowControl|FlipFlop
    (:A
      (Audio|Components|Audio|Play _audio 0.0)
      (if (Variables|Default|GetLongLift)
        (bind _z (Timeline|Timeline Play)
          (:Update
            (Transformation|SetWorldLocation (Variables|Default|GetStaticMesh) (Math|Vector|Lerp(Vector) (Transformation|GetWorldLocation (Variables|Default|GetStartLocation)) (Transformation|GetWorldLocation (Variables|Default|GetTargetLocation)) _z) false false))
          (:Finished
            (Audio|Components|Audio|Stop (Variables|Default|GetAudio))))
        (else
          (bind _z_2 (Timeline|UPDown Play)
            (:Update
              (Transformation|SetWorldLocation (Variables|Default|GetStaticMesh) (Math|Vector|Lerp(Vector) (Transformation|GetWorldLocation (Variables|Default|GetStartLocation)) (Transformation|GetWorldLocation (Variables|Default|GetTargetLocation)) _z_2) false false))
            (:Finished
              (Audio|Components|Audio|Stop (Variables|Default|GetAudio)))))))
    (:B
      (Audio|Components|Audio|Play _audio 0.0)
      (Timeline|UPDown Reverse))))

(fn ConstructionScript
  (|CallParentFunction))